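; BP_UnitMeshComponent is a unit's skeletal mesh component that performs a locked-out attack when Interact is triggered.
; On BeginPlay it replaces its first material with a dynamic instance.
; Interact, if not locked, darkens BodyColor, sets AttackLocked and plays the AM_Attack montage.
; When the montage completes, a WeaponRecoveryTime delay precedes restoring a lighter color and unlocking the attack.
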(event EventBeginPlay
  (bind _returnvalue (Rendering|Material|CreateDynamicMaterialInstance (Rendering|Material|GetMaterial 0) "None" :!class /Script/Engine.KismetMaterialLibrary))
  (bind _output_get (Variables|Material|SetDynamicMaterialInstance _returnvalue))
  (Rendering|Material|SetMaterial 0 _output_get))

(event EventTick
  (params (DeltaSeconds :type Float%20%28single-precision%29)))

(event EventInteract
  (if (not (Variables|Default|GetAttackLocked))
    (Rendering|Material|SetVectorParameterValue (Variables|Material|GetDynamicMaterialInstance) "BodyColor" "(R=0.191667,G=0.135851,B=0.191667,A=0.000000)" :!class /Script/Engine.MaterialInstanceDynamic)
    (Variables|Default|SetAttackLocked true)
    (Animation|Montage|PlayMontage self "/Game/Animations/Mixamo/Retargets/AM_Attack.AM_Attack"
      (:OnCompleted
        (Utilities|FlowControl|Delay (Variables|Default|GetWeaponRecoveryTime))
        (Rendering|Material|SetVectorParameterValue (Variables|Material|GetDynamicMaterialInstance) "BodyColor" "(R=0.701102,G=0.496933,B=0.701102,A=0.000000)" :!class /Script/Engine.MaterialInstanceDynamic)
        (Variables|Default|SetAttackLocked false)))))