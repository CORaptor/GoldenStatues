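; Player character for grid-based movement with mouse-driven interaction, a Health component that receives damage, and input disabled on death.
; Forward and right input events compute an adjacent-field destination, spawn a BP_Block there and call SimpleMoveToLocation.
; A cursor trace with a camera distance check switches to a hand cursor over Interactable objects, and left click messages the component or actor.
; EvaluateMovement offers a blocking line trace but is never called here.
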(event OnDie(Health)
  (Input|DisableInput (Game|GetPlayerController 0)))

(event EventTick
  (params (DeltaSeconds :type Float%20%28single-precision%29))
  (bind _returnvalue (Game|GetPlayerController 0))
  (bind (_hitresult_hitactor _hitresult_hitcomponent _inreach) (CallFunction|TraceforObjectsinMouseReach))
  (if _inreach
    (if (or (Utilities|DoesObjectImplementInterface _hitresult_hitactor "/Script/GoldenStatues.Interactable") (Utilities|DoesObjectImplementInterface _hitresult_hitcomponent "/Script/GoldenStatues.Interactable"))
      (Variables|/Script/Engine.PlayerController|SetCurrentMouseCursor _returnvalue "Hand")
      (else
        (Variables|/Script/Engine.PlayerController|SetCurrentMouseCursor _returnvalue "Default" :!label _label)))
    (else
      (goto _label))))

(event Collision|EventActorBeginOverlap
  (params (OtherActor :type Actor%20Object%20Reference)))

(event Game|Damage|EventAnyDamage
  (params (Damage :type Float%20%28single-precision%29) (DamageType :type Damage%20Type%20Object%20Reference) (InstigatedBy :type Controller%20Object%20Reference) (DamageCauser :type Actor%20Object%20Reference))
  (Class|HealthComponent|TakeDamage (Variables|Default|GetHealth) Damage))

(event EventMoveForwardEvent
  (params (Value :type Float%20%28single-precision%29))
  (CallFunction|MovetoAdjacentField Value (Math|Vector|GetForwardVector (Transformation|GetActorRotation))))

(event EventMoveRightEvent
  (params (Value :type Float%20%28single-precision%29))
  (CallFunction|MovetoAdjacentField Value (Math|Vector|GetRightVector (Transformation|GetActorRotation))))

(event EventBeginPlay
  (Variables|/Script/Engine.PlayerController|SetbShowMouseCursor (Game|GetPlayerController 0) true))

(event Input|MouseEvents|LeftMouseButton
  (params (Key :type Key%20Structure :default "None"))
  (:Pressed
    (bind (_hitresult_hitactor _hitresult_hitcomponent _inreach) (CallFunction|TraceforObjectsinMouseReach))
    (bind _interactable (Utilities|GetInteractableUnderCursor _hitresult_hitactor _hitresult_hitcomponent _inreach)
      (:Succeeded
        (Class|Interactable|Interact(Message) _interactable)))))

(fn ConstructionScript)

(fn MovetoAdjacentField
  (params (Value :type Float%20%28single-precision%29) (DirectionVector :type Vector))
  (bind _destination (CallFunction|CalculateDestination Value DirectionVector))
  (Game|SpawnActorfromClass "/Game/Blueprints/BP_Block.BP_Block_C" (Math|Transform|MakeTransform _destination "0, 0, 0" "1,1,1") "Undefined" 0 0)
  (AI|Navigation|SimpleMovetoLocation (Pawn|GetController) _destination))

(fn EvaluateMovement
  (params (DirectionVector :type Vector :default "0, 0, 0") (Sign :type Float%20%28single-precision%29))
  (bind _returnvalue (Transformation|GetActorLocation))
  (bind _returnvalue_2 (Collision|LineTraceByChannel _returnvalue (+ _returnvalue (* DirectionVector (* (Variables|Default|GetGridSize) Sign))) "TraceTypeQuery1" false 0 "None"))
  (return (not _returnvalue_2)))

(fn TraceforObjectsinMouseReach
  (bind _returnvalue (Game|GetPlayerController 0))
  (bind _hitresult (Game|Player|GetHitResultUnderCursorbyChannel _returnvalue "TraceTypeQuery3" true))
  (return (.hitactor _hitresult) (.hitcomponent _hitresult) (<= (Math|Vector|Distance(Vector) (Transformation|GetWorldLocation (Variables|Default|GetFollowCamera)) (.location _hitresult)) 5e+02)))

(fn CalculateDestination
  (params (Value :type Float%20%28single-precision%29) (DirectionVector :type Vector))
  (return (+ (Transformation|GetActorLocation) (* DirectionVector (+ (* (+ (Variables|Default|GetGridSize) (LocalVariables|GetToleranceCorrection)) (Math|Float|Sign(Float) Value)) (Variables|Default|GetGridOffset))))))