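; Player character that moves between grid fields and interacts with objects by mouse click.
; Forward and right move events feed MoveToAdjacentField, which line-traces one grid step and, if clear, issues SimpleMoveToLocation with offset and tolerance correction.
; A left click traces under the always-visible cursor and sends InteractMessage to Interactable actors whose hit point is within 500 units of the follow camera.
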(event Collision|EventActorBeginOverlap
  (params (OtherActor :type Actor%20Object%20Reference)))

(event EventMoveForwardEvent
  (params (Value :type Float%20%28single-precision%29))
  (CallFunction|MovetoAdjacentField Value (Math|Vector|GetForwardVector (Transformation|GetActorRotation))))

(event EventMoveRightEvent
  (params (Value :type Float%20%28single-precision%29))
  (CallFunction|MovetoAdjacentField Value (Math|Vector|GetRightVector (Transformation|GetActorRotation))))

(event EventBeginPlay
  (Variables|/Script/Engine.PlayerController|SetbShowMouseCursor (Game|GetPlayerController 0) true))

(event Input|MouseEvents|LeftMouseButton
  (params (Key :type Key%20Structure :default "None"))
  (bind _returnvalue (Game|GetPlayerController 0))
  (bind _hitresult (Game|Player|GetHitResultUnderCursorbyChannel _returnvalue "TraceTypeQuery1" true))
  (:Pressed
    (if (and (<= (Math|Vector|Distance(Vector) (Transformation|GetWorldLocation (Variables|Default|GetFollowCamera)) (.location _hitresult)) 5e+02) (Utilities|DoesObjectImplementInterface (.hitactor _hitresult) "/Script/GoldenStatues.Interactable"))
      (Class|Interactable|Interact(Message) (.hitactor _hitresult)))))

(fn ConstructionScript)

(fn MovetoAdjacentField
  (params (Value :type Float%20%28single-precision%29) (DirectionVector :type Vector))
  (bind _returnvalue (Transformation|GetActorLocation))
  (bind _returnvalue_2 (Math|Float|Sign(Float) Value))
  (bind _returnvalue_3 (Collision|LineTraceByChannel _returnvalue (+ _returnvalue (* DirectionVector (* (Variables|Default|GetGridSize) _returnvalue_2))) "TraceTypeQuery1" false 0 "None"))
  (if (not _returnvalue_3)
    (AI|Navigation|SimpleMovetoLocation (Pawn|GetController) (+ (Transformation|GetActorLocation) (* DirectionVector (+ (* (+ (Variables|Default|GetGridSize) (LocalVariables|GetToleranceCorrection)) _returnvalue_2) (Variables|Default|GetGridOffset)))))))